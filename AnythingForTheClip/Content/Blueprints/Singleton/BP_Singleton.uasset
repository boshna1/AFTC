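; BP_Singleton holds shared game state: objective progress, exit availability, viewer and subscriber counts, and audio volumes.
; On Init it waits briefly, records unique BP_IO_BaseItem transforms and uses their count as the objective total.
; Reaching that total unlocks the exit and shows it on the player HUD, while CollectObj grows subs and viewers by random, scaling amounts.
; StartVariables applies default sprint, lean, FOV and raycast settings to the player character.
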(event EventInit
  (Utilities|FlowControl|Delay 1.0)
  (bind _outactors (Actor|GetAllActorsOfClass "/Game/Blueprints/Environment/Interactables/Items/BP_IO_BaseItem.BP_IO_BaseItem_C"))
  (for _array_element _outactors
    (Utilities|Array|AddUnique (Variables|Default|GetSpawnLocations) (Transformation|GetActorTransform _array_element)))
  (CallFunction|SetTObjs))

(fn StartVariables
  (Development|PrintString "fire init" true true "(R=0.000000,G=0.660000,B=1.000000,A=1.000000)" 5.0)
  (bind _asbp_player_character (Utilities|Casting|CastToBP_PlayerCharacter (Game|Player|GetPlayerPawn 0)))
  (Utilities|FlowControl|Sequence
    (:then_0
      (Development|PrintString "fire init" true true "(R=0.000000,G=0.660000,B=1.000000,A=1.000000)" 5.0)
      (Variables|/Game/Blueprints/Player/BP_PlayerCharacter.BP_PlayerCharacter_C|SetLeanAmount _asbp_player_character 0.0)
      (Variables|/Game/Blueprints/Player/BP_PlayerCharacter.BP_PlayerCharacter_C|SetTimeToGainSprint _asbp_player_character 1.65)
      (Variables|/Game/Blueprints/Player/BP_PlayerCharacter.BP_PlayerCharacter_C|SetSprintResource _asbp_player_character 5e+02)
      (Variables|/Game/Blueprints/Player/BP_PlayerCharacter.BP_PlayerCharacter_C|SetSprintValue _asbp_player_character 1e+03)
      (Variables|/Game/Blueprints/Player/BP_PlayerCharacter.BP_PlayerCharacter_C|SetWalkValue _asbp_player_character 6e+02)
      (Variables|/Game/Blueprints/Player/BP_PlayerCharacter.BP_PlayerCharacter_C|SetTargetLean _asbp_player_character 0.0)
      (Variables|/Game/Blueprints/Player/BP_PlayerCharacter.BP_PlayerCharacter_C|SetSprintReduceAmount _asbp_player_character 2.0)
      (Variables|/Game/Blueprints/Player/BP_PlayerCharacter.BP_PlayerCharacter_C|SetSprintGainAmount _asbp_player_character 0.8)
      (Variables|/Game/Blueprints/Player/BP_PlayerCharacter.BP_PlayerCharacter_C|SetDefaultFov _asbp_player_character 1.2e+02)
      (Variables|/Game/Blueprints/Player/BP_PlayerCharacter.BP_PlayerCharacter_C|SetSprintFov _asbp_player_character 1.3e+02)
      (Variables|/Game/Blueprints/Player/BP_PlayerCharacter.BP_PlayerCharacter_C|Set0Fov _asbp_player_character 9e+01)
      (Variables|/Game/Blueprints/Player/BP_PlayerCharacter.BP_PlayerCharacter_C|SetRayCastDist _asbp_player_character 2e+02))))

(fn SetObjectives
  (params (Input :type Integer))
  (bind _output_get (Variables|Default|SetObjectivesGot (+ Input (Variables|Default|GetObjectivesGot))))
  (if (== _output_get (Variables|Default|GetTotalOBJS))
    (Variables|Default|SetCanExit true)
    (bind _asbp_player_character (Utilities|Casting|CastToBP_PlayerCharacter (Game|Player|GetPlayerPawn 0)))
    (Default|ShowExit (Variables|/Game/Blueprints/Player/BP_PlayerCharacter.BP_PlayerCharacter_C|GetMainHudRef _asbp_player_character))))

(fn GetObjectivesGot
  (return (Variables|Default|GetObjectivesGot)))

(fn SetViewers
  (params (AddViewers :type Integer))
  (Variables|Default|SetViewers (+ (Variables|Default|GetViewers) AddViewers)))

(fn GetViewers
  (return (Variables|Default|GetViewers)))

(fn SetSubs
  (params (AddSubs :type Integer))
  (Variables|Default|SetSubs (+ (Variables|Default|GetSubs) AddSubs)))

(fn GetSubs
  (return (Variables|Default|GetSubs)))

(fn CollectObj
  (CallFunction|SetSubs (Math|Random|RandomIntegerinRange (Math|Float|Truncate (+ (* (Variables|Default|GetSubs) 1.2) 1.0)) (Math|Float|Truncate (+ (* (Variables|Default|GetSubs) 1.3) 12.0))))
  (CallFunction|SetViewers (Math|Random|RandomIntegerinRange (Math|Float|Truncate (+ (* (Math|Conversions|ToFloat(Integer) (Variables|Default|GetViewers)) 1.1) 1.0)) (Math|Float|Truncate (+ (* (Math|Conversions|ToFloat(Integer) (Variables|Default|GetViewers)) 1.6) 7e+01)))))

(fn GetCanExit
  (return (Variables|Default|GetCanExit)))

(fn SetTObjs
  (Variables|Default|SetTotalOBJS (Utilities|Array|Length (Variables|Default|GetSpawnLocations))))

(fn SetVolumes
  (params (MasterVol :type Float%20%28double-precision%29) (SFXVol :type Float%20%28double-precision%29) (MusicVol :type Float%20%28double-precision%29))
  (Variables|Default|SetMasterVol MasterVol)
  (Variables|Default|SetSFXVol SFXVol)
  (Variables|Default|SetMusicVol MusicVol))

(fn GetVolumes
  (return (Variables|Default|GetMasterVol) (Variables|Default|GetSFXVol) (Variables|Default|GetMusicVol)))