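; BP_Entity is an AI creature that roams wander points and hunts the player through an enum state machine: Wander, Investigate, Alert, Chase, Search and Transform.
; Tick runs each state's AI moves and timers, while SetState changes walk speed.
; Line-of-sight traces switch Alert to Chase or Investigate, and Chase to Search at the last seen position.
; Perception and blackboard hooks are stubs that never change state.
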(event OnTargetPerceptionUpdated(AIPerception)
  (params (Actor :type Actor%20Object%20Reference) (Stimulus :type AI%20Stimulus%20Structure))
  (Class|AIPerceptionSystem|GetSenseClassforStimulus Stimulus))

(event Custom|Behavior)

(event Custom|ReEnableWander
  ;[0.15 0.15 0.15 0.5] Investigate Sequence 2 | checks if enum is equivalent | then checks if its far enough from its distance (by this point assigned by the sound/player detected in non-immediate range) if so move to the destination | After a delay after reaching the destination and not detecting another sound/player go back to investigate
  (if (Utilities|Enum|Equal(Enum) (Variables|Default|GetState) "NewEnumerator1")
    (CallFunction|SetState "NewEnumerator0")))

(event Custom|AlertCheck
  ;[0.15 0.15 0.15 0.5] Alert Sequence 3 | Checks if enum is equivalent | creates ray towards target, if the ray hits a player, and after a delay, stays true set enum to chase | Otherwise set player last seen variable and go to it and set enum to investigate clear target
  (bind _outhit (Collision|LineTraceByChannel (+ (Transformation|GetActorLocation) "0.000000,0.000000,80.000000") (Transformation|GetActorLocation (Variables|Default|GetTargetPoint)) "TraceTypeQuery1" false 0 "ForOneFrame"))
  (bind _asbp_player_character (Utilities|Casting|CastToBP_PlayerCharacter (.HitActor (Collision|BreakHitResult _outhit)))
    (:then
      (bind _output_get (Variables|Default|SetTargetPoint _asbp_player_character))
      (bind _output_get_2 (Variables|Default|SetDestination (Transformation|GetActorLocation _output_get)))
      (Variables|Default|SetPlayerLastSeen _output_get_2)
      (Utilities|Time|ClearandInvalidateTimerbyHandle (Variables|Default|GetActiveTimer))
      (CallFunction|SetState "NewEnumerator3"))
    (:CastFailed
      (Variables|Default|SetDestination "0, 0, 0")
      (Utilities|Time|ClearandInvalidateTimerbyHandle (Variables|Default|GetActiveTimer))
      (CallFunction|SetState "NewEnumerator1")
      (Variables|Default|SetTargetPoint 0))))

(event Custom|SetWanderPoint
  (AI|Components|Blackboard|SetValueasVector (AI|GetBlackboard 0) (Variables|Default|GetWanderPoint) (Variables|Default|GetDestination)))

(event Custom|ChaseCheck
  ;[0.15 0.15 0.15 0.5] Chase Sequence 4 | Checks if enum is equivalent | Creates ray towards player, if LOS is broken after 0.5 seconds go to last seen destination | if recast is valid keep moving
  (Development|PrintString "check chase")
  (bind _outhit (Collision|LineTraceByChannel (+ (Transformation|GetActorLocation) "0.000000,0.000000,80.000000") (Transformation|GetActorLocation (Game|Player|GetPlayerPawn 0)) "TraceTypeQuery1" false 0 "ForOneFrame"))
  (bind _asbp_player_character (Utilities|Casting|CastToBP_PlayerCharacter (.HitActor (Collision|BreakHitResult _outhit)))
    (:then
      (Utilities|Time|ClearandInvalidateTimerbyHandle (Variables|Default|GetActiveTimer))
      (bind _output_get (Variables|Default|SetTargetPoint _asbp_player_character))
      (bind _output_get_2 (Variables|Default|SetDestination (Transformation|GetActorLocation _output_get)))
      (Variables|Default|SetPlayerLastSeen _output_get_2)
      (AI|AIMoveTo self (Variables|Default|GetDestination) (Variables|Default|GetTargetPoint) 1e+01 false
        (:OnSuccess
          (CallFunction|ChaseCheck))))
    (:CastFailed
      (Variables|Default|SetDestination (Variables|Default|GetPlayerLastSeen))
      (Variables|Default|SetPlayerLastSeen "0, 0, 0")
      (Utilities|Time|ClearandInvalidateTimerbyHandle (Variables|Default|GetActiveTimer))
      (CallFunction|SetState "NewEnumerator4")
      (Variables|Default|SetTargetPoint 0))))

(event Custom|SetSearch
  ;[0.15 0.15 0.15 0.5] Search Sequence 5 | Checksi f enum is equivalent | if entity is far enough from player last seen location keep moving towards | if not go back to wandering
  (if (Utilities|Enum|Equal(Enum) (Variables|Default|GetState) "NewEnumerator4")
    (CallFunction|SetState "NewEnumerator0")))

(event EventBeginPlay
  ;[0.15 0.15 0.15 0.5] BeginPlay - after a delay, to inherit info from spawner, Executes SetWander and SetState
  (Utilities|FlowControl|Delay 1.0)
  (CallFunction|SetWander)
  (CallFunction|SetState "NewEnumerator0"))

(event Collision|EventActorBeginOverlap
  (params (OtherActor :type Actor%20Object%20Reference)))

(event EventTick
  (params (DeltaSeconds :type Float%20%28single-precision%29))
  (Utilities|FlowControl|Sequence
    (:then_0
      ;[0.15 0.15 0.15 0.5] Wander Sequence 1 - first checks if enum is equivalent | if true and actor is far enough from its destination, assign a new target, then
      (if (Utilities|Enum|Equal(Enum) (Variables|Default|GetState) "NewEnumerator0")
        (AI|AIMoveTo self (Variables|Default|GetDestination) (Variables|Default|GetTargetPoint) 1e+01 false
          (:OnSuccess
            (CallFunction|SetWander)
            (CallFunction|SetState "NewEnumerator0")))))
    (:then_1
      ;[0.15 0.15 0.15 0.5] Investigate Sequence 2 | checks if enum is equivalent | then checks if its far enough from its distance (by this point assigned by the sound/player detected in non-immediate range) if so move to the destination | After a delay after reaching the destination and not detecting another sound/player go back to investigate
      (if (Utilities|Enum|Equal(Enum) (Variables|Default|GetState) "NewEnumerator1")
        (AI|AIMoveTo self (Variables|Default|GetDestination) 0 1e+01 false
          (:OnSuccess
            (bind _returnvalue (Utilities|Time|SetTimerbyEvent (delegate Custom|ReEnableWander) 0.8))
            (Variables|Default|SetActiveTimer _returnvalue)))))
    (:then_2
      ;[0.15 0.15 0.15 0.5] Alert Sequence 3 | Checks if enum is equivalent | creates ray towards target, if the ray hits a player, and after a delay, stays true set enum to chase | Otherwise set player last seen variable and go to it and set enum to investigate clear target
      (if (Utilities|Enum|Equal(Enum) (Variables|Default|GetState) "NewEnumerator2")
        (bind _returnvalue_2 (Utilities|Time|SetTimerbyEvent (delegate Custom|AlertCheck) 0.8))
        (Variables|Default|SetActiveTimer _returnvalue_2)))
    (:then_3
      ;[0.15 0.15 0.15 0.5] Chase Sequence 4 | Checks if enum is equivalent | Creates ray towards player, if LOS is broken after 0.5 seconds go to last seen destination | if recast is valid keep moving
      (if (Utilities|Enum|Equal(Enum) (Variables|Default|GetState) "NewEnumerator3")
        (Development|PrintString "chase start")
        (bind _returnvalue_3 (Utilities|Time|SetTimerbyEvent (delegate Custom|ChaseCheck) 0.3 true false 0.0 3.0))
        (Development|PrintString "timer created")
        (Variables|Default|SetActiveTimer _returnvalue_3)))
    (:then_4
      ;[0.15 0.15 0.15 0.5] Search Sequence 5 | Checksi f enum is equivalent | if entity is far enough from player last seen location keep moving towards | if not go back to wandering
      (if (Utilities|Enum|Equal(Enum) (Variables|Default|GetState) "NewEnumerator4")
        (AI|AIMoveTo self (Variables|Default|GetDestination) 0 1e+01 false
          (:OnSuccess
            (Utilities|Time|SetTimerbyEvent (delegate Custom|SetSearch) 0.8)))))
    (:then_5
      (Utilities|FlowControl|Delay 0.5)
      (Development|PrintString (Utilities|String|EnumtoString (Variables|Default|GetState))))
    (:then_6
      (if (Utilities|Enum|Equal(Enum) (Variables|Default|GetState) "NewEnumerator5")
        (Utilities|FlowControl|Delay 3.0)
        (CallFunction|SetState "NewEnumerator3")))))

(fn ConstructionScript)

(fn SetState
  (params (State :type E_Entity_States%20Enum :default "NewEnumerator0"))
  ;[0.15 0.15 0.15 0.5] SetState - Sets the enum variable to the inputted state and then according to which one it is, sets variables
  (Utilities|Time|ClearandInvalidateTimerbyHandle (Variables|Default|GetActiveTimer))
  (bind _output_get (Variables|Default|SetState State))
  (switch Utilities|FlowControl|Switch|SwitchonE_Entity_States _output_get
    (:NewEnumerator0
      (CallFunction|VariableStates 6e+02))
    (:NewEnumerator1
      (CallFunction|VariableStates 8.5e+02))
    (:NewEnumerator2
      (CallFunction|VariableStates 1e+03))
    (:NewEnumerator3
      (CallFunction|VariableStates 1.5e+03))
    (:NewEnumerator4
      (CallFunction|VariableStates 1e+03))
    (:NewEnumerator5
      (CallFunction|VariableStates 0.0)))
  (CallFunction|Behavior))

(fn VariableStates
  (params (Speed :type Float%20%28double-precision%29) (Mesh :type Skeletal%20Mesh%20Object%20Reference))
  ;[0.15 0.15 0.15 0.5] VariableStates - Sets variables according to what input parameters are available
  (Variables|/Script/Engine.CharacterMovementComponent|SetMaxWalkSpeed (Variables|Character|GetCharacterMovement) Speed)
  (Variables|Default|SetEntityMesh Mesh))

(fn SetWander
  ;[0.15 0.15 0.15 0.5] Generates a random integer = length of target point length - 1
  (Variables|Default|SetRandomVar (Math|Random|RandomInteger (Utilities|Array|Length (Variables|Default|GetWanderPoints))) :!label _label)
  (if (== (Utilities|Array|Get(acopy) (Variables|Default|GetWanderPoints) (Variables|Default|GetRandomVar)) (Variables|Default|GetTargetPoint))
    (goto _label)
    (else
      ;[0.15 0.15 0.15 0.5] Sets TargetPoint Variable (object reference of the entity's destination) according to the randomize and also the destination variable which is a bector type
      (Variables|Default|SetTargetPoint (Utilities|Array|Get(acopy) (Variables|Default|GetWanderPoints) (Variables|Default|GetRandomVar)))
      (Variables|Default|SetDestination (Transformation|GetActorLocation (Utilities|Array|Get(acopy) (Variables|Default|GetWanderPoints) (Variables|Default|GetRandomVar)))))))