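; BP_Whispers is an ambient sound actor that periodically plays a random whisper-style sound around the player.
; On BeginPlay it finds the level's BP_AudioManager and starts a looping, delayed timer.
; Each tick of that timer picks one of four sounds and plays it through the manager at a low random volume.
; Placement is a random, positive-only offset from the player controller's location, not the pawn's.
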(event Custom|RandomSound
  (bind _returnvalue (Math|Random|RandomFloatinRange 0.0 5e+01))
  (bind _returnvalue_2 (Math|Random|RandomFloatinRange 0.0 2e+03))
  (bind _returnvalue_3 (Math|Random|RandomFloatinRange 0.0 2e+03))
  (bind _returnvalue_4 (Math|Random|RandomFloatinRange 0.0 0.2))
  (bind _returnvalue_5 (Game|GetPlayerController 0))
  (bind _audiomanager (Variables|Default|GetAudioManager))
  (bind _returnvalue_6 (Transformation|GetActorLocation _returnvalue_5))
  (bind _returnvalue_7 (Math|Vector|MakeVector _returnvalue_2 _returnvalue_3 _returnvalue))
  (bind _returnvalue_8 (+ _returnvalue_7 _returnvalue_6))
  (switch int (Math|Random|RandomInteger 4)
    (:0
      (Default|PlaySound _audiomanager "NewEnumerator7" _returnvalue_4 1.0 _returnvalue_8))
    (:1
      (Default|PlaySound _audiomanager "NewEnumerator8" _returnvalue_4 1.0 _returnvalue_8))
    (:2
      (Default|PlaySound _audiomanager "NewEnumerator9" (- _returnvalue_4 0.1) 1.0 _returnvalue_8))
    (:3
      (Default|PlaySound _audiomanager "NewEnumerator5" _returnvalue_4 1.0 _returnvalue_8))))

(event EventBeginPlay
  (bind _returnvalue (Actor|GetActorOfClass "/Game/Blueprints/Singleton/BP_AudioManager.BP_AudioManager_C"))
  (Variables|Default|SetAudioManager _returnvalue)
  (Utilities|Time|SetTimerbyEvent (delegate Custom|RandomSound) 8e+01 true false 6e+01))

(event Collision|EventActorBeginOverlap
  (params (OtherActor :type Actor%20Object%20Reference)))

(event EventTick
  (params (DeltaSeconds :type Float%20%28single-precision%29)))

(fn ConstructionScript)