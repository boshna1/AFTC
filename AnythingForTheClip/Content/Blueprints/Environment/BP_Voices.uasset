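; BP_Voices is an ambient sound actor that scatters random noises around the player.
; BeginPlay starts a looping one-second timer that calls SoundLoop.
; Each call randomly picks a metal drop, object drop, thunder or whisper FMOD event and plays it at low volume near the player pawn.
; The random horizontal offset only uses positive X and Y, so sounds always fall in one world-space quadrant.
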(event Custom|SoundLoop
  (bind _returnvalue (Game|Player|GetPlayerPawn 0))
  (bind _returnvalue_2 (Math|Random|RandomFloatinRange 0.0 5e+02))
  (bind _returnvalue_3 (Math|Random|RandomFloatinRange 0.0 5e+02))
  (bind _returnvalue_4 (Math|Vector|MakeVector _returnvalue_3 _returnvalue_2 0.0))
  (bind _returnvalue_5 (Transformation|GetActorLocation _returnvalue))
  (bind _returnvalue_6 (+ _returnvalue_5 _returnvalue_4))
  (switch int (Math|Random|RandomInteger 4)
    (:0
      (bind _returnvalue_7 (Class|FMODBlueprintStatics|PlayEventatLocation "/Game/FMOD/Banks/Events/Metal_Drop.Metal_Drop" (Math|Conversions|ToTransform(Vector) _returnvalue_6)))
      (Class|FMODBlueprintStatics|EventInstanceSetVolume _returnvalue_7 0.1))
    (:1
      (bind _returnvalue_8 (Class|FMODBlueprintStatics|PlayEventatLocation "/Game/FMOD/Banks/Events/Object_Drop.Object_Drop" (Math|Conversions|ToTransform(Vector) _returnvalue_6)))
      (Class|FMODBlueprintStatics|EventInstanceSetVolume _returnvalue_8 0.2))
    (:2
      (bind _returnvalue_9 (Class|FMODBlueprintStatics|PlayEventatLocation "/Game/FMOD/Banks/Events/Thunder.Thunder" (Math|Conversions|ToTransform(Vector) _returnvalue_6)))
      (Class|FMODBlueprintStatics|EventInstanceSetVolume _returnvalue_9 0.2))
    (:3
      (bind _returnvalue_10 (Class|FMODBlueprintStatics|PlayEventatLocation "/Game/FMOD/Banks/Events/Whisper.Whisper" (Math|Conversions|ToTransform(Vector) _returnvalue_6)))
      (Class|FMODBlueprintStatics|EventInstanceSetVolume _returnvalue_10 0.2))))

(event EventBeginPlay
  (Utilities|Time|SetTimerbyEvent (delegate Custom|SoundLoop) 1.0 true))

(event Collision|EventActorBeginOverlap
  (params (OtherActor :type Actor%20Object%20Reference)))

(event EventTick
  (params (DeltaSeconds :type Float%20%28single-precision%29)))

(fn ConstructionScript)