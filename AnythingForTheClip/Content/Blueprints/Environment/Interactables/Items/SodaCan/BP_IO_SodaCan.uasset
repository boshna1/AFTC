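; Interactable soda can item that gives each spawned instance a randomized material.
; On BeginPlay it sets its Model to Soda, creates a dynamic material instance from CanMaterial on the Cube component, and randomizes three scalar parameters on it.
; It then calls the parent BeginPlay, with no other active logic of its own.
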(event EventBeginPlay
  (Variables|Default|SetModel "/Game/Assets/Models/Items/SodaCan/Soda.Soda")
  (bind _returnvalue (Rendering|Material|CreateDynamicMaterialInstance (Variables|Default|GetCube) 0 "/Game/Assets/Models/Items/SodaCan/CanMaterial.CanMaterial" "None" :!class /Script/Engine.PrimitiveComponent))
  (bind _output_get (Variables|Default|SetMaterial _returnvalue))
  (Rendering|Material|SetScalarParameterValue _output_get "Param1" (Math|Random|RandomFloatinRange 0.1 2e+01) :!class /Script/Engine.MaterialInstanceDynamic)
  (Rendering|Material|SetScalarParameterValue _output_get "Param2" (Math|Random|RandomFloatinRange 0.1 2e+01) :!class /Script/Engine.MaterialInstanceDynamic)
  (Rendering|Material|SetScalarParameterValue _output_get "Param3" (Math|Random|RandomFloatinRange 0.1 2e+01) :!class /Script/Engine.MaterialInstanceDynamic)
  (|CallParentFunction))

(event Collision|EventActorBeginOverlap
  (params (OtherActor :type Actor%20Object%20Reference))
  (|CallParentFunction OtherActor) ; This node is disabled and will not be called.\nDrag off pins to build functionality.
)

(event EventTick
  (params (DeltaSeconds :type Float%20%28single-precision%29))
  (|CallParentFunction DeltaSeconds) ; This node is disabled and will not be called.\nDrag off pins to build functionality.
)

(fn ConstructionScript
  (|CallParentFunction))