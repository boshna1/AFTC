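; Base Blueprint for interactable physics items that can be picked up and released.
; PickUp sets the passed Root's Cube as the physics constraint's second component and, if that is valid, moves its own Cube to the given position.
; Break sets the Cube's linear velocity from the offset between its Velocity input and the last PickUp position, divided by Tick's delta time, imparting motion on release.
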(event Custom|PickUp
  (params (Root :type BP%20Player%20Character%20Object%20Reference) (NewPos :type Vector))
  (bind _cube (Variables|/Game/Blueprints/Player/BP_PlayerCharacter.BP_PlayerCharacter_C|GetCube Root))
  (Class|PhysicsConstraintComponent|SetConstrainedComponents (Variables|Default|GetPhysicsConstraint) 0 "None" _cube "None")
  (Utilities|IsValid _cube
    (:Is%20Valid
      (Transformation|SetWorldLocation (Variables|Default|GetCube) NewPos false false))))

(event Custom|Break
  (params (Velocity :type Vector))
  (Physics|SetPhysicsLinearVelocity (Variables|Default|GetCube) (/ (- Velocity (stale Custom|PickUp NewPos)) (stale EventTick DeltaSeconds)) false "None"))

(event EventBeginPlay)

(event Collision|EventActorBeginOverlap
  (params (OtherActor :type Actor%20Object%20Reference)))

(event EventTick
  (params (DeltaSeconds :type Float%20%28single-precision%29)))

(fn ConstructionScript)