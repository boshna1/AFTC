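; First-person player character handling movement, stamina-based sprint, toggle leaning, pause menu, backpack attach/detach and held-item carrying.
; Tick drives stamina, exhaustion breathing, interpolated camera roll and FOV, plus the camera trace used to grab and move items.
; Looping timers play footsteps and emit tagged noise through MakeNoise.
; Hitting BP_Entity moves the camera onto a spawned death camera; hitting BP_Exit only prints a win if exit is allowed.
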(event OnComponentHit(CapsuleComponent)
  (params (HitComponent :type Primitive%20Component%20Object%20Reference) (OtherActor :type Actor%20Object%20Reference) (OtherComp :type Primitive%20Component%20Object%20Reference) (NormalImpulse :type Vector :default "0, 0, 0") (Hit :type Hit%20Result%20Structure%20%28by%20ref%29))
  (Utilities|FlowControl|Sequence
    (:then_0
      (Utilities|Casting|CastToBP_Entity OtherActor)
      (Utilities|Time|SetTimerbyFunctionName 0 "DeathCam" 0.01 true))
    (:then_1
      (Utilities|Casting|CastToBP_Exit OtherActor)
      (bind _asbp_singleton (Utilities|Casting|CastToBP_Singleton (Game|GetGameInstance)))
      (bind _condition (Default|GetCanExit _asbp_singleton))
      (if _condition
        (Development|PrintString "WIn")))))

(event Custom|StartGainSprint
  ;[0.15 0.15 0.15 0.5] Sprint
  ;;[0.15 0.15 0.15 0.5] When stopped sprinting, first sets movespeed back to walking speed, then starts timer. when timer completes player starts gaining sprint
  (Variables|Default|SetGainSprint true)
  (Variables|Default|SetPlayBreathingSound true))

(event Custom|RunningSound
  (Default|PlaySound (Variables|Default|GetAudioManager) "NewEnumerator11" 1.0 1.0 (Transformation|GetActorLocation))
  (Class|Actor|MakeNoise 1.0 0 "0, 0, 0" 5e+01 "SprintStep"))

(event Custom|DeathCam
  (bind _camera (Variables|Default|GetCamera))
  (bind _capsulecomponent (Variables|Collision|GetCapsuleComponent))
  (if (not (Variables|Default|GetCreateCam))
    (Transformation|DetachFromComponent _camera "KeepWorld" "KeepWorld" "KeepWorld" true)
    (Variables|Default|SetCreateCam true)
    (bind _returnvalue (Game|SpawnActorfromClass "/Game/Blueprints/Player/BP_DeathCamera.BP_DeathCamera_C" (Transformation|GetActorTransform) "Undefined" "MultiplyWithRoot" 0 0))
    (Transformation|AttachComponentToComponent _camera (Variables|/Game/Blueprints/Player/BP_DeathCamera.BP_DeathCamera_C|GetCube _returnvalue) "None" "SnapToTarget" "SnapToTarget" "SnapToTarget" true)
    (Pawn|Components|CharacterMovement|DisableMovement (Variables|Character|GetCharacterMovement))
    (Collision|SetCollisionEnabled _capsulecomponent "NoCollision")
    (Physics|SetSimulatePhysics _capsulecomponent true)
    (Input|DisableInput (Game|GetPlayerController 0))
    (bind _returnvalue_2 (Actor|GetActorOfClass "/Game/Blueprints/Entity/BP_Entity.BP_Entity_C"))
    (Transformation|AttachActorToActor _returnvalue_2 "None" "SnapToTarget" "SnapToTarget" "SnapToTarget" true)
    (Utilities|Time|ClearandInvalidateTimerbyHandle (Variables|Default|GetHandleTimer))))

(event Custom|WalkSound
  (Default|PlaySound (Variables|Default|GetAudioManager) "NewEnumerator11" 1.0 1.0 (Transformation|GetActorLocation))
  (Class|Actor|MakeNoise 0.4 0 "0, 0, 0" 2e+01 "WalkStep"))

(event Custom|TriggerPause
  (bind _returnvalue (Game|GetPlayerController 0))
  (bind _returnvalue_2 (Game|GetPlayerController 0))
  (bind _mainhudref (Variables|Default|GetMainHudRef))
  (Utilities|IsValid (Variables|Default|GetPauseUI)
    (:Is%20Valid
      (Default|ClearWidget (Variables|Default|GetPauseUI))
      (Widget|RemovefromParent (Variables|Default|GetPauseUI))
      (Variables|Default|SetPauseUI 0)
      (Variables|/Script/Engine.PlayerController|SetbShowMouseCursor _returnvalue false)
      (Input|SetInputModeGameOnly _returnvalue false)
      (bind _output_get (Variables|Default|SetIsPaused false))
      (Default|SetPause/Play _mainhudref _output_get)
      (Game|SetGamePaused _output_get))
    (:Is%20Not%20Valid
      (bind _returnvalue_3 (UserInterface|CreateWidget "/Game/Blueprints/UI/BPW_UI_Pause.BPW_UI_Pause_C"))
      (bind _output_get_2 (Variables|Default|SetPauseUI _returnvalue_3))
      (UserInterface|Viewport|AddtoViewport _output_get_2 0)
      (Variables|/Script/Engine.PlayerController|SetbShowMouseCursor _returnvalue_2 true)
      (Input|SetInputModeUIOnly _returnvalue_2 (Variables|Default|GetPauseUI) "DoNotLock" false)
      (bind _output_get_3 (Variables|Default|SetIsPaused true))
      (Default|SetPause/Play _mainhudref _output_get_3)
      (Game|SetGamePaused _output_get_3))))

(event Custom|StartWalkSound
  (bind _returnvalue (Utilities|Time|SetTimerbyEvent (delegate Custom|WalkSound) 0.5 true))
  (Variables|Default|SetHandleTimer _returnvalue))

(event Input|EnhancedActionEvents|EnhancedInputActionIA_Lean
  (params (ActionValue :type Float%20%28double-precision%29) (ElapsedSeconds :type Float%20%28double-precision%29) (TriggeredSeconds :type Float%20%28double-precision%29) (InputAction :type Input%20Action%20Object%20Reference :default "/Game/Blueprints/Player/Input/IA_Lean.IA_Lean"))
  ;[0.15 0.15 0.15 0.5] Lean Logic - action value = 1/-1 depending on Q/E press | Checks if Lean amount is 0 and is full leaning then if lean press is the same as current lean, if so reset camera. | If lean input is not the same lean other way | if lean amount is != 0 check if already leaning, if so check if camera is reset, if so reset variables | if not leaning set lean to true and lean towards key press
  (if (and (and (Variables|Default|GetIsFullLean) (or (!= (Variables|Default|GetLeanAmount) 15.0) (!= (Variables|Default|GetLeanAmount) -15.0))) (!= (Variables|Default|GetLeanAmount) 0.0))
    (if (== (Variables|Default|GetLeanMod) ActionValue)
      (Variables|Default|SetTargetLean 0.0)
      (Variables|Default|SetLeanMod 0.0)
      (Variables|Default|SetIsLeaning true)
      (else
        (Variables|Default|SetTargetLean (* ActionValue 15.0))
        (Variables|Default|SetLeanMod ActionValue)))
    (elif (Variables|Default|GetIsLeaning)
      (if (not (!= (Variables|Default|GetLeanAmount) 0.0))
        (Variables|Default|SetIsLeaning false)
        (Variables|Default|SetIsFullLean false))
      (else
        (Variables|Default|SetIsLeaning true)
        (if (== ActionValue -1.0)
          (Variables|Default|SetLeanMod -1.0)
          (Variables|Default|SetTargetLean -15.0)
          (else
            (Variables|Default|SetLeanMod 1.0)
            (Variables|Default|SetTargetLean 15.0)))))))

(event Input|EnhancedActionEvents|EnhancedInputActionIA_Look
  (params (ActionValue :type Vector%202D%20Structure) (ElapsedSeconds :type Float%20%28double-precision%29) (TriggeredSeconds :type Float%20%28double-precision%29) (InputAction :type Input%20Action%20Object%20Reference :default "/Game/Blueprints/Player/Input/IA_Look.IA_Look"))
  (bind (_x _y) (Math|Vector2D|BreakVector2D ActionValue))
  ;[0.15 0.15 0.15 0.5] Look
  (Pawn|Input|AddControllerYawInput _x)
  (Pawn|Input|AddControllerPitchInput _y))

(event Input|EnhancedActionEvents|EnhancedInputActionIA_Move
  (params (ActionValue :type Vector%202D%20Structure) (ElapsedSeconds :type Float%20%28double-precision%29) (TriggeredSeconds :type Float%20%28double-precision%29) (InputAction :type Input%20Action%20Object%20Reference :default "/Game/Blueprints/Player/Input/IA_Move.IA_Move"))
  (bind (_x _y) (Math|Vector2D|BreakVector2D ActionValue))
  ;[0.15 0.15 0.15 0.5] Movement
  (:Triggered
    (Pawn|Input|AddMovementInput (Transformation|GetActorRightVector) _x false)
    (Pawn|Input|AddMovementInput (Transformation|GetActorForwardVector) _y false))
  (:Started
    (Variables|Default|SetIsWalking true :!label _label)
    (Variables|Default|SetPlayWalkingSound true)
    (Variables|Default|SetPlaySprintBreathe true)
    (if (Variables|Default|GetPlayWalkingSound)
      (if (Variables|Default|GetIsWalking)
        (bind _returnvalue (Utilities|Time|SetTimerbyEvent (delegate Custom|WalkSound) 0.5 true))
        (Variables|Default|SetHandleTimer _returnvalue))))
  (:Ongoing
    (goto _label))
  (:Completed
    (Variables|Default|SetIsWalking false)
    (Variables|Default|SetIsSprinting false)
    (Variables|Default|SetPlaySprintingSound false)
    (Variables|Default|SetPlayWalkingSound false)
    (Variables|Default|SetPlaySprintBreathe false)
    (Utilities|Time|ClearandInvalidateTimerbyHandle (Variables|Default|GetHandleTimer))))

(event Input|EnhancedActionEvents|EnhancedInputActionIA_LeftClick
  (params (ActionValue :type Boolean) (ElapsedSeconds :type Float%20%28double-precision%29) (TriggeredSeconds :type Float%20%28double-precision%29) (InputAction :type Input%20Action%20Object%20Reference :default "/Game/Blueprints/Player/Input/IA_LeftClick.IA_LeftClick"))
  (:Started
    (Variables|Default|SetIsHolding true)
    (bind _asbp_io_base_item (Utilities|Casting|CastToBP_IO_BaseItem (.HitActor (Collision|BreakHitResult (stale EventTick _outhit)))))
    (Variables|Default|SetHoldTarget _asbp_io_base_item)
    (Physics|SetSimulatePhysics (Variables|/Game/Blueprints/Environment/Interactables/Items/BP_IO_BaseItem.BP_IO_BaseItem_C|GetCube _asbp_io_base_item) false))
  (:Completed
    (Variables|Default|SetIsHolding false)
    (Physics|SetSimulatePhysics (Variables|/Game/Blueprints/Environment/Interactables/Items/BP_IO_BaseItem.BP_IO_BaseItem_C|GetCube _asbp_io_base_item) true)
    (Variables|Default|SetHoldTarget 0)))

(event Input|EnhancedActionEvents|EnhancedInputActionIA_Sprint
  (params (ActionValue :type Boolean) (ElapsedSeconds :type Float%20%28double-precision%29) (TriggeredSeconds :type Float%20%28double-precision%29) (InputAction :type Input%20Action%20Object%20Reference :default "/Game/Blueprints/Player/Input/IA_Sprint.IA_Sprint"))
  ;[0.15 0.15 0.15 0.5] Sprint
  (:Started
    ;;[0.15 0.15 0.15 0.5] OnSprint being pressed checks if sprint resource > 0 then sets new movespeed and disables gaining sprint
    (Utilities|Time|ClearandInvalidateTimerbyHandle (Variables|Default|GetHandleTimer))
    (Variables|Default|SetPlayWalkingSound true))
  (:Ongoing
    (if (> (Variables|Default|GetSprintResource) 0.0)
      (Variables|Default|SetGainSprint false)
      (Variables|Default|SetMoveSpeed (Variables|Default|GetSprintValue))
      (Variables|Default|SetIsSprinting true)
      (else
        (Utilities|Time|ClearandInvalidateTimerbyHandle (Variables|Default|GetHandleTimer))
        ;;[0.15 0.15 0.15 0.5] When stopped sprinting, first sets movespeed back to walking speed, then starts timer. when timer completes player starts gaining sprint
        (Variables|Default|SetMoveSpeed (Variables|Default|GetWalkValue) :!label _label)
        (Variables|Default|SetIsSprinting false)))
    (Variables|/Script/Engine.CharacterMovementComponent|SetMaxWalkSpeed (Variables|Character|GetCharacterMovement) (Variables|Default|GetMoveSpeed))
    (if (Variables|Default|GetPlaySprintingSound)
      (bind _returnvalue (Utilities|Time|SetTimerbyEvent (delegate Custom|RunningSound) 0.35 true))
      (Variables|Default|SetHandleTimer _returnvalue)
      (Variables|Default|SetPlaySprintingSound false)))
  (:Completed
    (Utilities|FlowControl|Sequence
      (:then_0
        (goto _label))
      (:then_1
        (Utilities|Time|SetTimerbyEvent (delegate Custom|StartGainSprint) (Variables|Default|GetTimeToGainSprint) false true))
      (:then_2
        (Utilities|Time|ClearandInvalidateTimerbyHandle (Variables|Default|GetHandleTimer))
        (Variables|Default|SetPlaySprintingSound true)
        (Variables|Default|SetPlayWalkingSound true)
        (if (Variables|Default|GetIsWalking)
          (CallFunction|StartWalkSound))))))

(event Input|EnhancedActionEvents|EnhancedInputActionIA_Esc
  (params (ActionValue :type Boolean) (ElapsedSeconds :type Float%20%28double-precision%29) (TriggeredSeconds :type Float%20%28double-precision%29) (InputAction :type Input%20Action%20Object%20Reference :default "/Game/Blueprints/Player/Input/IA_Esc.IA_Esc"))
  (bind _returnvalue (Game|GetPlayerController 0))
  (bind _returnvalue_2 (Game|GetPlayerController 0))
  (bind _mainhudref (Variables|Default|GetMainHudRef))
  (:Started
    (Utilities|IsValid (Variables|Default|GetPauseUI)
      (:Is%20Valid
        (Default|ClearWidget (Variables|Default|GetPauseUI))
        (Widget|RemovefromParent (Variables|Default|GetPauseUI))
        (Variables|Default|SetPauseUI 0)
        (Variables|/Script/Engine.PlayerController|SetbShowMouseCursor _returnvalue false)
        (Input|SetInputModeGameOnly _returnvalue false)
        (bind _output_get (Variables|Default|SetIsPaused false))
        (Default|SetPause/Play _mainhudref _output_get)
        (Game|SetGamePaused _output_get))
      (:Is%20Not%20Valid
        (bind _returnvalue_3 (UserInterface|CreateWidget "/Game/Blueprints/UI/BPW_UI_Pause.BPW_UI_Pause_C"))
        (bind _output_get_2 (Variables|Default|SetPauseUI _returnvalue_3))
        (UserInterface|Viewport|AddtoViewport _output_get_2 0)
        (Variables|/Script/Engine.PlayerController|SetbShowMouseCursor _returnvalue_2 true)
        (Input|SetInputModeUIOnly _returnvalue_2 (Variables|Default|GetPauseUI) "DoNotLock" false)
        (bind _output_get_3 (Variables|Default|SetIsPaused true))
        (Default|SetPause/Play _mainhudref _output_get_3)
        (Game|SetGamePaused _output_get_3)))))

(event Input|EnhancedActionEvents|EnhancedInputActionIA_Backpack
  (params (ActionValue :type Boolean) (ElapsedSeconds :type Float%20%28double-precision%29) (TriggeredSeconds :type Float%20%28double-precision%29) (InputAction :type Input%20Action%20Object%20Reference :default "/Game/Blueprints/Player/Input/IA_Backpack.IA_Backpack"))
  (bind _backpackref (Variables|Default|GetBackpackRef))
  (:Started
    (if (Variables|Default|GetHasBackpack)
      (Variables|Default|SetHasBackpack false)
      (Default|Detach _backpackref)
      (elif (not (> (Math|Vector|Distance2D(Vector) (Transformation|GetActorLocation) (Transformation|GetActorLocation (Variables|Default|GetBackpackRef))) 1.5e+02))
        (Variables|Default|SetHasBackpack true)
        (Default|Attach _backpackref)))))

(event EventBeginPlay
  (bind _returnvalue (Game|GetPlayerController 0))
  ;[0.15 0.15 0.15 0.5] BeginPlay
  (Utilities|FlowControl|Sequence
    (:then_0
      ;;[0.15 0.15 0.15 0.5] Add Mapping Context
      (bind _asplayer_controller (Utilities|Casting|CastToPlayerController (Game|GetPlayerController 0)))
      (Utilities|IsValid (PlayerController|LocalPlayerSubsystems|GetEnhancedInputLocalPlayerSubsystem _asplayer_controller)
        (:Is%20Valid
          (Input|AddMappingContext (PlayerController|LocalPlayerSubsystems|GetEnhancedInputLocalPlayerSubsystem _asplayer_controller) "/Game/Blueprints/Player/Input/IMC_Game_Player.IMC_Game_Player" 0 "(bIgnoreAllPressedKeysUntilRelease=True,bForceImmediately=False,bNotifyUserSettings=False)")
          (if (not (Class|EnhancedInputUserSettings|IsMappingContextRegistered (Class|EnhancedInputSubsystemInterface|GetUserSettings (PlayerController|LocalPlayerSubsystems|GetEnhancedInputLocalPlayerSubsystem _asplayer_controller)) "/Game/Blueprints/Player/Input/IMC_Game_Player.IMC_Game_Player"))
            (Class|EnhancedInputUserSettings|RegisterInputMappingContext (Class|EnhancedInputSubsystemInterface|GetUserSettings (PlayerController|LocalPlayerSubsystems|GetEnhancedInputLocalPlayerSubsystem _asplayer_controller)) "/Game/Blueprints/Player/Input/IMC_Game_Player.IMC_Game_Player")))))
    (:then_1
      (bind _asbp_singleton (Utilities|Casting|CastToBP_Singleton (Game|GetGameInstance)))
      (Default|StartVariables _asbp_singleton))
    (:then_2
      (bind _returnvalue_2 (Actor|GetActorOfClass "/Game/Blueprints/Player/BP_Player_Backpack.BP_Player_Backpack_C"))
      (Variables|Default|SetBackpackRef _returnvalue_2))
    (:then_3
      (Physics|Components|PhysicsHandle|SetTargetLocation (Variables|Default|GetPhysicsHandle) (Transformation|GetWorldLocation (Variables|Default|GetSphere1))))
    (:then_4
      (bind _returnvalue_3 (UserInterface|CreateWidget "/Game/Blueprints/UI/BPW_MainHUD.BPW_MainHUD_C" (Game|GetPlayerController 0)))
      (UserInterface|Viewport|AddtoViewport _returnvalue_3 0)
      (Variables|Default|SetMainHudRef _returnvalue_3)
      (Input|SetInputModeGameOnly _returnvalue false)
      (Variables|/Script/Engine.PlayerController|SetbShowMouseCursor _returnvalue false))
    (:then_5
      (bind _returnvalue_4 (Actor|GetActorOfClass "/Game/Blueprints/Singleton/BP_AudioManager.BP_AudioManager_C"))
      (Variables|Default|SetAudioManager _returnvalue_4))))

(event Collision|EventActorBeginOverlap
  (params (OtherActor :type Actor%20Object%20Reference)))

(event EventTick
  (params (DeltaSeconds :type Float%20%28single-precision%29))
  (bind _returnvalue (Pawn|GetControlRotation :!class /Script/Engine.Pawn))
  (bind _returnvalue_2 (Game|GetPlayerController 0))
  (bind _returnvalue_3 (Pawn|GetControlRotation :!class /Script/Engine.Pawn))
  (bind _camera (Variables|Default|GetCamera))
  (bind _raycastdist (Variables|Default|GetRayCastDist))
  (bind (_roll _pitch _yaw) (Math|Rotator|BreakRotator _returnvalue))
  (bind _returnvalue_4 (Transformation|GetWorldLocation _camera))
  (bind _returnvalue_5 (Transformation|GetActorRotation _returnvalue_2))
  (bind (_roll_2 _pitch_2 _yaw_2) (Math|Rotator|BreakRotator _returnvalue_3))
  (bind _returnvalue_6 (Math|Vector|GetForwardVector _returnvalue_5))
  (bind _returnvalue_7 (* _returnvalue_6 _raycastdist))
  (bind _returnvalue_8 (+ _returnvalue_7 _returnvalue_4))
  ;[0.15 0.15 0.15 0.5] EventTick - if is sprinting reduce sprint resource by delta seconds + 2
  (Utilities|FlowControl|Sequence
    (:then_0
      (if (Variables|Default|GetIsSprinting)
        (Variables|Default|SetSprintResource (- (Variables|Default|GetSprintResource) (+ DeltaSeconds (Variables|Default|GetSprintReduceAmount))))))
    (:then_1
      ;[0.15 0.15 0.15 0.5] EventTick - Gain Sprint resource by delta seconds + 0.8 if able and isnt sprinting and resource is not greater than certain amount
      (if (Variables|Default|GetGainSprint)
        (if (not (Variables|Default|GetIsSprinting))
          (if (< (Variables|Default|GetSprintResource) 5e+02)
            (Variables|Default|SetSprintResource (+ (Variables|Default|GetSprintResource) (+ DeltaSeconds (Variables|Default|GetSprintGainAmount))))))))
    (:then_2
      ;[0.15 0.15 0.15 0.5] Checks if IsLeaning is active if so rotate the camera towards the target X (Roll) then activate full lean variable as long as the lean amount and target are equal and it isnt 0
      (if (Variables|Default|GetIsLeaning)
        (Variables|Default|SetLeanAmount (Math|Interpolation|FInterpTo (Variables|Default|GetLeanAmount) (Variables|Default|GetTargetLean) DeltaSeconds 12.0))
        (Transformation|SetWorldRotation (Variables|Default|GetCamSocket) (Math|Rotator|MakeRotator (Math|Interpolation|FInterpTo (Variables|Default|GetLeanAmount) (Variables|Default|GetTargetLean) DeltaSeconds 12.0) _pitch_2 _yaw_2) false false)
        (if (and (== (Variables|Default|GetLeanAmount) (Variables|Default|GetTargetLean)) (!= (Variables|Default|GetLeanAmount) 0.0))
          (Variables|Default|SetIsFullLean true)
          (Variables|Default|SetIsLeaning false))
        (else
          (Transformation|SetWorldRotation (Variables|Default|GetCamSocket) (Math|Rotator|MakeRotator (Variables|Default|GetLeanAmount) _pitch _yaw) false false))))
    (:then_3
      ;[0.15 0.15 0.15 0.5] Sprint Fov
      (if (Variables|Default|GetIsSprinting)
        (Variables|Default|SetTargetCameraFov (Variables|Default|GetSprintFov))
        (else
          (Variables|Default|SetTargetCameraFov (Variables|Default|GetDefaultFov))))
      (if (<= (Variables|Default|GetSprintResource) 0.0)
        (Variables|Default|SetTargetCameraFov (Variables|Default|Get0Fov))
        (if (Variables|Default|GetPlayBreathingSound)
          (Default|PlaySound (Variables|Default|GetAudioManager) "NewEnumerator1" 1.0 1.0 (Transformation|GetActorLocation))
          (Variables|Default|SetPlayBreathingSound false)))
      (bind _output_get (Variables|Default|SetCurrentCameraFov (Math|Interpolation|FInterpTo (Variables|Default|GetCurrentCameraFov) (Variables|Default|GetTargetCameraFov) DeltaSeconds 5.0)))
      (Camera|SetFieldOfView (Variables|Default|GetCamera) _output_get))
    (:then_4
      (bind _outhit (Collision|LineTraceByChannel _returnvalue_4 _returnvalue_8 "TraceTypeQuery1" false (Utilities|Array|MakeArray self 0) "ForOneFrame")))
    (:then_5
      (if (Variables|Default|GetIsHolding)
        (Transformation|SetWorldTransform (Variables|/Game/Blueprints/Environment/Interactables/Items/BP_IO_BaseItem.BP_IO_BaseItem_C|GetCube (stale Input|EnhancedActionEvents|EnhancedInputActionIA_LeftClick _asbp_io_base_item)) (Math|Transform|MakeTransform _returnvalue_8 "0, 0, 0" (.Scale (Math|Transform|BreakTransform (Transformation|GetRelativeTransform (Variables|/Game/Blueprints/Environment/Interactables/Items/BP_IO_BaseItem.BP_IO_BaseItem_C|GetCube (stale Input|EnhancedActionEvents|EnhancedInputActionIA_LeftClick _asbp_io_base_item)))))) false false)))))

(fn ConstructionScript)