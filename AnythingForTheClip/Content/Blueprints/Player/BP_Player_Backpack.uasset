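; Player backpack actor that collects BP_IO_BaseItem actors touching its box.
; On begin play it caches the object pool and attaches to the player's Sphere component; Detach drops it just above the ground found by a downward trace.
; Box overlap disables the item through the pool, updates objectives on the BP_Singleton game instance and calls the HUD's Collect.
; End overlap detaches items and removes them from HeldItems, but the code adding them is unwired.
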(event OnComponentBeginOverlap(Box)
  (params (OverlappedComponent :type Primitive%20Component%20Object%20Reference) (OtherActor :type Actor%20Object%20Reference) (OtherComp :type Primitive%20Component%20Object%20Reference) (OtherBodyIndex :type Integer) (bFromSweep :type Boolean) (SweepResult :type Hit%20Result%20Structure%20%28by%20ref%29))
  (bind _asbp_io_base_item (Utilities|Casting|CastToBP_IO_BaseItem OtherActor))
  (Default|DisableItem (Variables|Default|GetOBJPool) _asbp_io_base_item)
  (bind _asbp_singleton (Utilities|Casting|CastToBP_Singleton (Game|GetGameInstance)))
  (Default|SetObjectives _asbp_singleton 1)
  (bind _returnvalue (Actor|GetActorOfClass "/Game/Blueprints/Player/BP_PlayerCharacter.BP_PlayerCharacter_C"))
  (Default|Collect (Variables|/Game/Blueprints/Player/BP_PlayerCharacter.BP_PlayerCharacter_C|GetMainHudRef _returnvalue)))

(event OnComponentEndOverlap(Box)
  (params (OverlappedComponent :type Primitive%20Component%20Object%20Reference) (OtherActor :type Actor%20Object%20Reference) (OtherComp :type Primitive%20Component%20Object%20Reference) (OtherBodyIndex :type Integer))
  (bind _asbp_io_base_item (Utilities|Casting|CastToBP_IO_BaseItem OtherActor))
  (Utilities|Array|RemoveItem (Variables|Default|GetHeldItems) _asbp_io_base_item)
  (Transformation|DetachFromComponent (Variables|/Script/Engine.Actor|GetRootComponent _asbp_io_base_item) "KeepWorld" "KeepWorld" "KeepWorld" true))

(event EventBeginPlay
  (bind _returnvalue (Actor|GetActorOfClass "/Game/Blueprints/Player/BP_OBJPool.BP_OBJPool_C"))
  (Variables|Default|SetOBJPool _returnvalue)
  (CallFunction|Attach)
  (bind _returnvalue_2 (Actor|GetActorOfClass "/Game/Blueprints/Player/BP_PlayerCharacter.BP_PlayerCharacter_C"))
  (Utilities|Array|Add (Variables|Default|GetActorsToIgnore) _returnvalue_2))

(event Collision|EventActorBeginOverlap
  (params (OtherActor :type Actor%20Object%20Reference)))

(event EventTick
  (params (DeltaSeconds :type Float%20%28single-precision%29)))

(fn ConstructionScript)

(fn Attach
  (bind _asbp_player_character (Utilities|Casting|CastToBP_PlayerCharacter (Game|Player|GetPlayerPawn 0)))
  (Transformation|AttachComponentToComponent (Variables|/Game/Blueprints/Player/BP_PlayerCharacter.BP_PlayerCharacter_C|GetSphere _asbp_player_character) "None" "KeepRelative" "KeepRelative" "KeepRelative" false)
  (Transformation|SetActorLocation (Transformation|GetWorldLocation (Variables|/Game/Blueprints/Player/BP_PlayerCharacter.BP_PlayerCharacter_C|GetSphere _asbp_player_character)) false false)
  (for _array_element (Variables|Default|GetHeldItems) :!label _label
    (Transformation|SetActorLocation _array_element (Transformation|GetWorldLocation (Variables|/Game/Blueprints/Player/BP_PlayerCharacter.BP_PlayerCharacter_C|GetSphere _asbp_player_character)) false false)
    (goto _label)))

(fn Detach
  (bind _returnvalue (Transformation|GetActorLocation))
  (Transformation|DetachFromActor self "KeepWorld" "KeepWorld" "KeepWorld")
  (bind _outhit (Collision|LineTraceByChannel _returnvalue (+ _returnvalue "0.000000,0.000000,-1000.000000") "TraceTypeQuery1" false (Variables|Default|GetActorsToIgnore) "ForOneFrame"))
  (Transformation|SetActorLocation (+ (.ImpactPoint (Collision|BreakHitResult _outhit)) "0.000000,0.000000,40.000000") false true))