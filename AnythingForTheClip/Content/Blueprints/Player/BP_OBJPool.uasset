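; BP_OBJPool pools BP_IO_BaseItem items, recycling them by teleporting instead of spawning or destroying.
; Shortly after BeginPlay it caches SpawnLocations from the BP_Singleton game instance and registers all existing items as enabled.
; DisableItem parks items high at a fixed point in AvailablePool; EnableItem returns them to EnabledPool.
; NewWave enables available items at index-matched spawn locations, though EnableItem shrinks the array being iterated.
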(event EventBeginPlay
  (Utilities|FlowControl|Delay 1.1)
  (bind _asbp_singleton (Utilities|Casting|CastToBP_Singleton (Game|GetGameInstance)))
  (Variables|Default|SetSpawnLocations (Variables|/Game/Blueprints/Singleton/BP_Singleton.BP_Singleton_C|GetSpawnLocations _asbp_singleton))
  (bind _outactors (Actor|GetAllActorsOfClass "/Game/Blueprints/Environment/Interactables/Items/BP_IO_BaseItem.BP_IO_BaseItem_C"))
  (Variables|Default|SetEnabledPool _outactors))

(event Collision|EventActorBeginOverlap
  (params (OtherActor :type Actor%20Object%20Reference)))

(event EventTick
  (params (DeltaSeconds :type Float%20%28single-precision%29)))

(fn ConstructionScript)

(fn AssignNewItems
  (params (Item :type BP%20IO%20Base%20Item%20Object%20Reference))
  (Utilities|Array|AddUnique (Variables|Default|GetEnabledPool) Item))

(fn EnableItem
  (params (Item :type BP%20IO%20Base%20Item%20Object%20Reference) (Location :type Vector))
  (Utilities|Array|RemoveItem (Variables|Default|GetAvailablePool) Item)
  (Utilities|Array|AddUnique (Variables|Default|GetEnabledPool) Item)
  (Transformation|SetActorLocation Item Location false true))

(fn DisableItem
  (params (Item :type BP%20IO%20Base%20Item%20Object%20Reference))
  (Utilities|Array|RemoveItem (Variables|Default|GetEnabledPool) Item)
  (Utilities|Array|AddUnique (Variables|Default|GetAvailablePool) Item)
  (Transformation|SetActorLocation Item "0.000000,0.000000,8000.000000" false true))

(fn NewWave
  (for (_array_element _array_index) (Variables|Default|GetAvailablePool)
    (CallFunction|EnableItem _array_element (.Location (Math|Transform|BreakTransform (Utilities|Array|Get(acopy) (Variables|Default|GetSpawnLocations) _array_index))))))